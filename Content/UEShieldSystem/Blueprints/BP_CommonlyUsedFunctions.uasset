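; Shared helper functions for vision-cone queries and line traces in the shield system.
; ConeVectorTrace filters all actors of a class by distance and dot-product angle, line traces to each, and returns unobstructed hits with trace lengths, optionally drawing the cone.
; ForwardLineTrace runs a complex object-type trace along a rotation's forward vector, scaling Length by 1000.
; ActorWithinAngle exposes the same forward-angle test as a standalone check.
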(fn `ActorWithinAngle`
  (params (ActorContext :type "Actor Object Reference") (Self :type "Actor Object Reference") (Angle :type "Float (double-precision)"))
  (returns (ActorWithinAngle :type Boolean))
  ;[1 1 1] Checks whether actor is within defined angle
  (return (< (`KismetMathLibrary.DegAcos` (`KismetMathLibrary.Dot_VectorVector` (`KismetMathLibrary.Normal` (- (`Actor.K2_GetActorLocation` ActorContext) (`Actor.K2_GetActorLocation` Self))) (`Actor.GetActorForwardVector` Self))) Angle)))

(fn `ConeVectorTrace`
  (params (OffsetConeStart :type "Vector Structure") (Actor :type "Actor Class Reference") (`Querying Actor` :type "Actor Object Reference") (`Trace Channel` :type "ETraceTypeQuery Enum" :default "TraceTypeQuery1") (`Trace Complex` :type Boolean) (`Draw Debug Type` :type "EDrawDebugTrace Enum" :default "None") (`Trace Colour` :type "LinearColor Structure") (`Trace Hit Colour` :type "LinearColor Structure") (ConeLength :type "Float (double-precision)") (`Cone Angle` :type "Float (double-precision)") (IgnoreList :type "Array of Actor Object Reference"))
  (returns (`Breask hit Results` :type "Array of HitResult Structure") (`Trace Lengths` :type "Array of Float (double-precision)"))
  (locals (HitResultStructure :type "Array of HitResult Structure") (ConeStart :type "Vector Structure") (TraceLength :type "Array of Float (double-precision)"))
  (bind _returnvalue (`Actor.K2_GetActorLocation` `Querying Actor`))
  (bind _returnvalue_2 (`Actor.GetActorForwardVector` `Querying Actor`))
  (bind _returnvalue_3 (+ OffsetConeStart _returnvalue))
  ;[1 1 1] Searches for an Actor of class within a specified cone and returns hit results once all actors have been line traced
  (bind _outactors (`GameplayStatics.GetAllActorsOfClass` null Actor))
  (for _array_element _outactors
    (set `local.ConeStart` _returnvalue_3)
    (bind _returnvalue_4 (`Actor.K2_GetActorLocation` _array_element))
    (bind _returnvalue_5 (- _returnvalue_4 _returnvalue))
    (if (<= (`KismetMathLibrary.VSize` _returnvalue_5) ConeLength)
      (if (< (`KismetMathLibrary.DegAcos` (`KismetMathLibrary.Dot_VectorVector` (`KismetMathLibrary.Normal` _returnvalue_5) _returnvalue_2)) `Cone Angle`)
        (bind _outhit (`KismetSystemLibrary.LineTraceSingle` null (`local.ConeStart`) _returnvalue_4 `Trace Channel` `Trace Complex` IgnoreList `Draw Debug Type` true `Trace Colour` `Trace Hit Colour`))
        (bind (_bblockinghit _binitialoverlap _time _distance _location _impactpoint _normal _impactnormal _physmat _hitactor _hitcomponent _hitbonename _hititem _faceindex _tracestart _traceend) (`GameplayStatics.BreakHitResult` _outhit))
        (if (== _array_element _hitactor)
          (`KismetArrayLibrary.Array_AddUnique` (`local.HitResultStructure`) _outhit)
          (`KismetArrayLibrary.Array_AddUnique` (`local.TraceLength`) (`KismetMathLibrary.VSize` (- _tracestart _traceend)))))))
  ;[1 1 1] Draw Debug cone
  (if (`|EnumInequality` `Draw Debug Type`)
    (`KismetSystemLibrary.DrawDebugConeInDegrees` null _returnvalue_3 _returnvalue_2 ConeLength `Cone Angle` `Cone Angle` 24 (struct :`R` 1.0 :`A` 1.0) 0.0 1.0))
  (return (`local.HitResultStructure`) (`local.TraceLength`)))

(fn `ForwardLineTrace`
  (params (`Querying Start Vector` :type "Vector Structure") (`Querying End Rotation` :type "Rotator Structure") (Length :type "Float (double-precision)") (`Object Types` :type "Array of EObjectTypeQuery Enum" :default _) (`Actors to ignore` :type "Array of Actor Object Reference") (`Draw Type` :type "EDrawDebugTrace Enum" :default "None"))
  (returns (`Hit Result` :type "HitResult Structure") (`Return Value` :type Boolean))
  ;[1 1 1] fires forward line trace
  (bind (_outhit _returnvalue) (`KismetSystemLibrary.LineTraceSingleForObjects` null `Querying Start Vector` (+ `Querying Start Vector` (* (`KismetMathLibrary.Conv_RotatorToVector` `Querying End Rotation`) (* 1000 Length))) `Object Types` true `Actors to ignore` `Draw Type`))
  (return _outhit _returnvalue))