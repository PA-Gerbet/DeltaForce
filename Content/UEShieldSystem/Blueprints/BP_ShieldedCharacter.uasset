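; Character Blueprint with a regenerating energy shield that absorbs damage before health, and ragdolls when health runs out.
; Hits drain the shield with an impact particle, or health once it is empty, then a retriggerable delay restarts the ShieldRegen timeline while alive.
; A dynamic material from the construction script maps shield strength to displacement, opacity, hue and emissive.
; Demo mode starts regen on BeginPlay; RestoreHealth self-repeats but is uncalled here.
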(event `RestoreHealth`
  ;[1 1 1] restores shields each cycle
  (if (>= (`self.Health`) 30.0)
    (set `self.Health` 30.0)
    (else
      (set `self.Health` (+ (`self.Health`) 2.0))
      (`KismetSystemLibrary.Delay` 0.2)
      (`self.RestoreHealth`))))

(event `self.ReceiveBeginPlay`
  ;[1 1 1] checks if character is in demo mode and begins shield regen
  (if (`self.Demo`)
    (`KismetSystemLibrary.Delay` 0.2)
    (if (!= (`self.ShieldStrength`) 50.0)
      (`self.RestoreShields`))))

(event `RestoreShields`
  ;[1 1 1] checks for damage imparted and then players shield regen timeline after a delay
  (bind (_direction _shieldlevel) (`Timeline|ShieldRegen` :!via `PlayFromStart` :!label _label)
    (:`Update`
      (set `self.ShieldStrength` _shieldlevel)
      (`self.UpdateShield`))))

(event `ReceieveDamage`
  (params (impactpoint :type "Vector Structure"))
  ;[1 1 1] checks for damage imparted and then players shield regen timeline after a delay
  (if (> (`self.ShieldStrength`) 0.0)
    (set `self.ShieldStrength` (- (`self.ShieldStrength`) 5.0))
    (`GameplayStatics.SpawnEmitterAtLocation` "/Game/UEShieldSystem/Particles/P_ShieldImpact.P_ShieldImpact" impactpoint)
    (`self.UpdateShield`)
    (else
      (`self.UpdateHealth`)))
  (`KismetSystemLibrary.RetriggerableDelay` 6.0)
  (if (> (`self.Health`) 0.0)
    (goto _label :!via `PlayFromStart`)))

(event `UpdateHealth`
  ;[1 1 1] checks for damage imparted and then players shield regen timeline after a delay
  (set `self.Health` (- (`self.Health`) 2.0))
  (if (<= (`self.Health`) 0.0)
    (`SkeletalMeshComponent.SetAllBodiesSimulatePhysics` (`self.Mesh`) true)))

(event `UpdateShield`
  (bind _dynamicshieldmaterial (`self.DynamicShieldMaterial`))
  (bind _dynamicshieldmaterial_2 (`self.DynamicShieldMaterial`))
  (bind _shieldstrength (`self.ShieldStrength`))
  ;[1 1 1] updates applicable shield material parameters
  (if (not (`KismetMathLibrary.InRange_FloatFloat` _shieldstrength -50.0 0.0))
    (`MaterialInstanceDynamic.SetScalarParameterValue` _dynamicshieldmaterial "Displacement Multiplier" (`KismetMathLibrary.MapRangeClamped` _shieldstrength 50.0 0.0 0.0 3.0))
    (`MaterialInstanceDynamic.SetScalarParameterValue` _dynamicshieldmaterial "Opacity" (`KismetMathLibrary.MapRangeClamped` _shieldstrength 50.0 1.0 0.0 1.0))
    (`MaterialInstanceDynamic.SetScalarParameterValue` _dynamicshieldmaterial "HueShift" (`KismetMathLibrary.MapRangeClamped` _shieldstrength 50.0 0.0 0.0 100.0)))
  (if (`KismetMathLibrary.InRange_FloatFloat` _shieldstrength -50.0 0.0)
    (`MaterialInstanceDynamic.SetScalarParameterValue` _dynamicshieldmaterial_2 "Emissive Strength" (`KismetMathLibrary.MapRangeClamped` _shieldstrength -50.0))
    (if (<= _shieldstrength 0.1)
      (`MaterialInstanceDynamic.SetScalarParameterValue` _dynamicshieldmaterial_2 "Opacity" (`KismetMathLibrary.MapRangeClamped` _shieldstrength -50.0)))
    (else
      (`MaterialInstanceDynamic.SetScalarParameterValue` _dynamicshieldmaterial_2 "Emissive Strength" 15.0))))

(fn `UserConstructionScript`
  (bind _shieldmaterial (`self.ShieldMaterial`))
  (bind _shieldstrength (`self.ShieldStrength`))
  (bind _mesh (`self.Mesh`))
  (bind _dynamicshieldmaterial (`self.DynamicShieldMaterial`))
  ;[1 1 1] creates and sets dynamic material instance
  (if (<= (`self.Health`) 0.0)
    (`PrimitiveComponent.SetSimulatePhysics` (`self.Mesh`) true))
  (`/Engine/EditorBlueprintResources/StandardMacros.IsValid` _shieldmaterial
    (:`Is Valid`
      (`PrimitiveComponent.SetMaterial` (`self.Mesh`) 1 _shieldmaterial))
    (:`Is Not Valid`
      _))
  (bind _returnvalue (`PrimitiveComponent.CreateDynamicMaterialInstance` _mesh 1 (`PrimitiveComponent.GetMaterial` _mesh 1)))
  ;[1 1 1] sets applicable shield parameters
  (set `self.DynamicShieldMaterial` _returnvalue)
  (`MaterialInstanceDynamic.SetScalarParameterValue` _dynamicshieldmaterial "Displacement Multiplier" (`KismetMathLibrary.MapRangeClamped` _shieldstrength 50.0 0.0 0.0 3.0))
  (`MaterialInstanceDynamic.SetScalarParameterValue` _dynamicshieldmaterial "Opacity" (`KismetMathLibrary.MapRangeClamped` _shieldstrength 50.0 1.0 0.0 1.0))
  (`MaterialInstanceDynamic.SetScalarParameterValue` _dynamicshieldmaterial "HueShift" (`KismetMathLibrary.MapRangeClamped` _shieldstrength 50.0 0.0 0.0 100.0))
  (if (`KismetMathLibrary.InRange_FloatFloat` 0.0 0.1)
    (`MaterialInstanceDynamic.SetScalarParameterValue` _dynamicshieldmaterial "Emissive Strength" (`KismetMathLibrary.MapRangeClamped` 0.0 1.0 0.1 0.0 1000.0))
    (if (<= _shieldstrength 0.1)
      (`MaterialInstanceDynamic.SetScalarParameterValue` _dynamicshieldmaterial "Opacity" (`KismetMathLibrary.MapRangeClamped` _shieldstrength 0.0 1.0))
      (if (!= (`self.ShieldStrength`) 50.0)
        (`self.RestoreShields`)))
    (else
      (`MaterialInstanceDynamic.SetScalarParameterValue` _dynamicshieldmaterial "Emissive Strength" 15.0))))