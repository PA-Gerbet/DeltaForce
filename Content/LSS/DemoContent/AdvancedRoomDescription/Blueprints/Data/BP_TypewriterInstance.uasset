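; BP_TypewriterInstance plays a typewriter text effect with typing sound on a text render component, part of the AdvancedRoomDescription demo content.
; Execute uses a Running flag to ignore calls while busy, clears the text and calls Run.
; Run proceeds only when wrap, visibility and the effect are enabled in TextSettings.
; A framerate-independent typewriter helper feeds characters and "<br>" breaks into AddStringToTextRender until completion.
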(event `Execute`
  (params (`Text Render` :type "TextRenderComponent Object Reference") (`Text Settings` :type "/Game/LSS/DemoContent/AdvancedRoomDescription/Blueprints/Data/S_WrappedTextRender Structure (by ref)"))
  (`/Engine/EditorBlueprintResources/StandardMacros.IsValid` `Text Render`
    (:`Is Valid`
      (if (not (`self.Running`))
        (set `self.Running` true)
        (`TextRenderComponent.K2_SetText` `Text Render` (`|FormatText` ""))
        (`self.Run` `Text Render` `Text Settings`
          (:`OutputPin`
            (set `self.Running` false)))))))

(fn `UserConstructionScript`)