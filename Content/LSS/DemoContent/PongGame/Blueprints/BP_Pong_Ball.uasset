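; Pong ball that launches along Y on BeginPlay and also handles scoring and the win check.
; Overlaps run a cast chain: paddles reverse Y and set X from paddle velocity plus random spread, while horizontal borders flip X.
; Goals re-center and relaunch the ball, increment the opposite score and update tagged TextRenderActors.
; Exceeding MaxScore prints the winner and sets Gameover, which this Blueprint never reads.
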(event `self.ReceiveBeginPlay`
  ;[1 1 1] Begin Here
  (`PrimitiveComponent.SetPhysicsLinearVelocity` (0.0 2000.0 0.0)))

(event `self.ReceiveActorBeginOverlap`
  (params (OtherActor :type "Actor Object Reference"))
  ;[1 1 1] Main Game Update
  (`self.Update Game` OtherActor))

(fn `Update Game`
  (params (InputPin :type "Actor Object Reference"))
  (bind _asbp_pong_player_r (cast `/Game/LSS/DemoContent/PongGame/Blueprints/BP_Pong_Player_R` InputPin)
    (:`then`
      (bind _returnvalue (`PrimitiveComponent.GetPhysicsLinearVelocity` _asbp_pong_player_r "None"))
      (bind _returnvalue_2 (`PrimitiveComponent.GetPhysicsLinearVelocity` "None"))
      (`PrimitiveComponent.SetPhysicsLinearVelocity` (`KismetMathLibrary.MakeVector` (+ (.x _returnvalue) (`KismetMathLibrary.RandomFloatInRange` -1000.0 1000.0)) (* (.y _returnvalue_2) -1.0) (.z _returnvalue_2)))
      (`GameplayStatics.PlaySoundAtLocation` "/Game/LSS/DemoContent/PongGame/Audio/S_ballCollision_Cue.S_ballCollision_Cue" (0.0 0.0 0.0) (struct) 1.0 1.0 0.0 null null null))
    (:`CastFailed`
      (bind _asbp_pong_player_l (cast `/Game/LSS/DemoContent/PongGame/Blueprints/BP_Pong_Player_L` InputPin)
        (:`then`
          (bind _returnvalue_3 (`PrimitiveComponent.GetPhysicsLinearVelocity` _asbp_pong_player_l "None"))
          (bind _returnvalue_4 (`PrimitiveComponent.GetPhysicsLinearVelocity` "None"))
          (`PrimitiveComponent.SetPhysicsLinearVelocity` (`KismetMathLibrary.MakeVector` (+ (.x _returnvalue_3) (`KismetMathLibrary.RandomFloatInRange` -1000.0 1000.0)) (* (.y _returnvalue_4) -1.0) (.z _returnvalue_4)))
          (`GameplayStatics.PlaySoundAtLocation` "/Game/LSS/DemoContent/PongGame/Audio/S_ballCollision_Cue.S_ballCollision_Cue" (0.0 0.0 0.0) (struct) 1.0 1.0 0.0 null null null))
        (:`CastFailed`
          (bind _asbp_pong_enemy (cast `/Game/LSS/DemoContent/PongGame/Blueprints/BP_Pong_Enemy` InputPin)
            (:`then`
              (bind _returnvalue_5 (`PrimitiveComponent.GetPhysicsLinearVelocity` _asbp_pong_enemy "None"))
              (bind _returnvalue_6 (`PrimitiveComponent.GetPhysicsLinearVelocity` "None"))
              (`PrimitiveComponent.SetPhysicsLinearVelocity` (`KismetMathLibrary.MakeVector` (+ (.x _returnvalue_5) (`KismetMathLibrary.RandomFloatInRange` -1000.0 1000.0)) (* (.y _returnvalue_6) -1.0) (.z _returnvalue_6)))
              (`GameplayStatics.PlaySoundAtLocation` "/Game/LSS/DemoContent/PongGame/Audio/S_ballCollision_Cue.S_ballCollision_Cue" (0.0 0.0 0.0) (struct) 1.0 1.0 0.0 null null null))
            (:`CastFailed`
              (cast `/Game/LSS/DemoContent/PongGame/Blueprints/BP_Pong_Border_H` InputPin
                (:`then`
                  (bind _returnvalue_7 (`PrimitiveComponent.GetPhysicsLinearVelocity` "None"))
                  (`PrimitiveComponent.SetPhysicsLinearVelocity` (`KismetMathLibrary.MakeVector` (* (.x _returnvalue_7) -1.0) (.y _returnvalue_7) (.z _returnvalue_7)))
                  (`GameplayStatics.PlaySoundAtLocation` "/Game/LSS/DemoContent/PongGame/Audio/S_ballCollision_Cue.S_ballCollision_Cue" (0.0 0.0 0.0) (struct) 1.0 1.0 0.0 null null null))
                (:`CastFailed`
                  (cast `/Game/LSS/DemoContent/PongGame/Blueprints/BP_Pong_Goal_L` InputPin
                    (:`then`
                      (`self.K2_SetActorLocation` (0.0 0.0 0.0))
                      (`PrimitiveComponent.SetPhysicsLinearVelocity` (0.0 2000.0 0.0))
                      (`GameplayStatics.PlaySoundAtLocation` "/Game/LSS/DemoContent/PongGame/Audio/S_ballGoal_Cue.S_ballGoal_Cue" (0.0 0.0 0.0) (struct) 1.0 1.0 0.0 null null null)
                      (set `self.RPlayer_Score` (+ (`self.RPlayer_Score`) 1))
                      (bind _outactors (`GameplayStatics.GetAllActorsOfClass` "/Script/Engine.TextRenderActor"))
                      (for _array_element _outactors
                        (bind _astext_render_actor (cast `TextRenderActor` _array_element))
                        (if (`ActorComponent.ComponentHasTag` _astext_render_actor "R_Player_Score_Tag")
                          (`TextRenderComponent.K2_SetText` (`TextRenderActor.TextRender` _astext_render_actor) (`KismetTextLibrary.Conv_IntToText` (`self.RPlayer_Score`)))
                          (if (> (`self.RPlayer_Score`) (`self.MaxScore`))
                            (`KismetSystemLibrary.PrintString` "Right side wins!")
                            (set `self.bGameover` true)))))
                    (:`CastFailed`
                      (cast `/Game/LSS/DemoContent/PongGame/Blueprints/BP_Pong_Goal_R` InputPin)
                      (`self.K2_SetActorLocation` (0.0 0.0 0.0))
                      (`PrimitiveComponent.SetPhysicsLinearVelocity` (0.0 -2000.0 0.0))
                      (`GameplayStatics.PlaySoundAtLocation` "/Game/LSS/DemoContent/PongGame/Audio/S_ballGoal_Cue.S_ballGoal_Cue" (0.0 0.0 0.0) (struct) 1.0 1.0 0.0 null null null)
                      (set `self.LPlayer_Score` (+ (`self.LPlayer_Score`) 1))
                      (bind _outactors_2 (`GameplayStatics.GetAllActorsOfClass` "/Script/Engine.TextRenderActor"))
                      (for _array_element_2 _outactors_2
                        (bind _astext_render_actor_2 (cast `TextRenderActor` _array_element_2))
                        (if (`ActorComponent.ComponentHasTag` _astext_render_actor_2 "L_Player_Score_Tag")
                          (`TextRenderComponent.K2_SetText` (`TextRenderActor.TextRender` _astext_render_actor_2) (`KismetTextLibrary.Conv_IntToText` (`self.LPlayer_Score`)))
                          (if (> (`self.LPlayer_Score`) (`self.MaxScore`))
                            (`KismetSystemLibrary.PrintString` "Left side wins!")
                            (set `self.bGameover` true)))))))))))))))

(fn `UserConstructionScript`)