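; Demo actor that displays the example LSS progress bar through a widget component, animated for show and not tied to real loading.
; On BeginPlay it casts the component's user widget and sets the progress bar's font size and fill image draw mode.
; A half-speed timeline then feeds its alpha, remapped to a percentage scale, into the widget's progress.
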(event `self.ReceiveBeginPlay`
  ;[1 1 1] Driving the percentage of the Widget via a timeline for demo purposes to show the widget (isn't hooked to actual loading)
  (`TimelineComponent.SetPlayRate` (`self.Animate Progress Bar`) 0.5)
  (bind _asui_lss_example_progress_bar (cast `/Game/LSS/UI/ExampleWidgets/UI_LSS_Example_ProgressBar` (`WidgetComponent.GetUserWidgetObject` (`self.UI Widget`))))
  (set `/Game/LSS/UI/ExampleWidgets/UI_LSS_Example_ProgressBar.Font Size` 20 _asui_lss_example_progress_bar)
  (`|VariableSetRef` (`.DrawAs` (break `SlateBrush` (`.FillImage` (break `ProgressBarStyle` (`ProgressBar.WidgetStyle` (`/Game/LSS/UI/ExampleWidgets/UI_LSS_Example_ProgressBar.ProgressBar_01` _asui_lss_example_progress_bar)))))) "Box")
  (bind (_direction _alpha) (`Timeline|Animate Progress Bar` :!via `PlayFromStart`)
    (:`Update`
      (`/Game/LSS/UI/ExampleWidgets/UI_LSS_Example_ProgressBar.Set Progress` _asui_lss_example_progress_bar (`KismetMathLibrary.MapRangeClamped` _alpha 0.0 1.0 0.0 100.0)))))

(fn `UserConstructionScript`)