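; BP_GunTurret is an AI gun turret that targets actors tagged Player.
; On BeginPlay it initializes its AITurretComponent with the roller, turret container, beam, overlap sphere and two secondary shoot points.
; That call also sets detection and attack ranges, pitch limits, rotation speed, free rotation and burst firing.
; The Blueprint adds no logic of its own to Tick or construction, which only call the parent.
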(event `self.ReceiveTick`
  (params (DeltaSeconds :type "Float (single-precision)"))
  (`parent.ReceiveTick` DeltaSeconds))

(event `self.ReceiveBeginPlay`
  (`parent.ReceiveBeginPlay`)
  ;[1 1 1] Init turret
  (`/Game/BP/AI/Turret/BP_AITurretComponent.Init` (`self.AITurretComponent`) false (`self.Roller`) (`self.TurretContainer`) (`|MakeArray` (`self.ShootPos`) (`self.ShootPos1`)) (`self.Beam`) 20000.0 17000.0 false -20.0 50.0 8.0 0 true false false 0.8 self true 4 0.2 false (`self.OverlapSphere`) "Player"))

(fn `UserConstructionScript`
  (`parent.UserConstructionScript`))