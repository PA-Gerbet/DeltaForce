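; Turret bullet projectile that travels forward, damages what it hits, and detonates any BP_RocketMain it strikes.
; Each Tick box-traces one frame of travel ahead, moving the actor only when nothing blocks it.
; Hits spawn a decal, push physics bodies and apply point damage once.
; Timelines stretch the mesh at spawn and shrink it with the light on impact or range expiry, while authority sets the actor lifespan.
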(event `self.ReceiveBeginPlay`
  ;[1 1 1] Create bullet
  (`GameplayStatics.PlaySoundAtLocation` (`self.ShotSound`) (`self.K2_GetActorLocation`) (struct) 1.0 1.0 0.0 null null null)
  (`KismetArrayLibrary.Array_Add` (`self.ActorsToIgnore`) (`self.Instigator`))
  (`|ExecutionSequence`
    (:`then_0`
      (`/Engine/EditorBlueprintResources/ActorMacros.Switch Has Authority`
        (:`Authority`
          (bind _output_get (set `self.MaxLife` (/ (`self.Range`) (`self.BulletSpeed`))))
          (`self.SetLifeSpan` (+ _output_get 3.0)))))
    (:`then_1`
      (bind (_direction _alpha) (`Timeline|Timeline_0`)
        (:`Update`
          (`SceneComponent.SetRelativeScale3D` (`self.StaticMesh`) (`KismetMathLibrary.MakeVector` 0.4 0.4 (`KismetMathLibrary.Lerp` 0.0 8.0 _alpha))))))))

(event `self.ReceiveTick`
  (params (DeltaSeconds :type "Float (single-precision)"))
  (bind _returnvalue (`self.K2_GetActorLocation`))
  (bind _staticmesh (`self.StaticMesh`))
  (bind _returnvalue_2 (* (* (`self.GetActorForwardVector`) (`self.BulletSpeed`)) DeltaSeconds))
  ;[1 1 1] Create trace from actor location + next frame location
  (bind _output_get (set `self.Life` (+ (`self.Life`) DeltaSeconds)))
  (if (<= _output_get (`self.MaxLife`))
    (bind _outhit (`KismetSystemLibrary.BoxTraceSingle` _returnvalue (+ _returnvalue _returnvalue_2) (30.0 10.0 10.0) (`self.K2_GetActorRotation`) "TraceTypeQuery1" true (`self.ActorsToIgnore`)))
    (bind (_bblockinghit _binitialoverlap _time _distance _location _impactpoint _normal _impactnormal _physmat _hitactor _hitcomponent _hitbonename _hititem _faceindex _tracestart _traceend) (`GameplayStatics.BreakHitResult` _outhit))
    (if _bblockinghit
      ;[1 1 1] If hit rocket, explode
      (bind _asbp_rocket_main (cast `/Game/BP/AI/Turret/BP_RocketMain` _hitactor)
        (:`then`
          (set `/Game/BP/AI/Turret/BP_RocketMain.AirPoof?` true _asbp_rocket_main)
          (bind _returnvalue_3 (`KismetMathLibrary.Conv_VectorToRotator` (* _impactnormal -1)))
          (`/Game/BP/AI/Turret/BP_RocketMain.Explode` _asbp_rocket_main self _returnvalue_3 (`self.K2_GetActorLocation`) _outhit false))
        (:`CastFailed`
          _))
      (`|ExecutionSequence`
        (:`then_0`
          (`GameplayStatics.SpawnDecalAttached` "/Game/Materials/MasterDecal_trans.MasterDecal_trans" (30.0 30.0 30.0) _hitcomponent "None" _impactpoint _returnvalue_3 "KeepRelativeOffset" 5.0) ; Create decal
          (if (`SceneComponent.IsSimulatingPhysics` _hitcomponent "None")
            (bind _returnvalue_4 (`KismetMathLibrary.Normal` (- _traceend _tracestart)))
            (`PrimitiveComponent.AddImpulse` _hitcomponent (* _returnvalue_4 (`self.PrimaryImpulseStrength`)) "None" false) ; Add impulse to hit actor
          )
          (`/Engine/EditorBlueprintResources/StandardMacros.DoOnce` false
            (:`Completed`
              (`GameplayStatics.ApplyPointDamage` _hitactor 4.0 _returnvalue_4 _outhit null self))))
        (:`then_1`
          ;[1 1 1] Set life time
          (set `self.Life` (+ (`self.MaxLife`) 1.0))))
      (`/Engine/EditorBlueprintResources/StandardMacros.DoOnce` false :!label _label
        (:`Completed`
          ;[1 1 1] Destroy bullet
          (bind (_direction _alpha) (`Timeline|Timeline_1` :!via `PlayFromStart`)
            (:`Update`
              (bind _returnvalue_5 (`KismetMathLibrary.Lerp` 0.4 0.0 _alpha))
              (`SceneComponent.SetRelativeScale3D` _staticmesh (`KismetMathLibrary.MakeVector` _returnvalue_5 _returnvalue_5 (`KismetMathLibrary.Lerp` 8.0 0.0 _alpha)))
              (`LightComponent.SetIntensity` (`self.PointLight`) (`KismetMathLibrary.Lerp` 4000.0 0.0 _alpha)))
            (:`Finished`
              (`SceneComponent.SetVisibility` _staticmesh false false)
              (`SceneComponent.SetVisibility` (`self.PointLight`) false false)))))
      (else
        ;[1 1 1] Move if not hited
        (`self.K2_AddActorWorldOffset` _returnvalue_2)))
    (else
      (goto _label))))

(fn `UserConstructionScript`)