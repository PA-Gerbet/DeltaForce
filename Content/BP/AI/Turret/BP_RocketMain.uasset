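; Configurable turret projectile that flies straight and deals point or radial damage, either bursting or staying stuck in what it hits.
; Tick sphere-traces one frame ahead, then moves or calls Explode, adding optional decals and detonating other rockets it hits.
; An anti-air timer or incoming point damage triggers an air burst.
; Explode applies damage and impulses, plays effects, then hides or attaches the mesh before a short lifespan.
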(event `AntiAirExplode`
  ;[1 1 1] Set explode timer for anti air rockets
  (`self.Explode` null (struct) (`self.K2_GetActorLocation`) (struct) true))

(event `self.ReceiveBeginPlay`
  ;[1 1 1] Set lifetime
  (`self.SetLifeSpan` (`self.Rocket Lifetime`))
  ;[1 1 1] Set explode timer for anti air rockets
  (if (`self.AntiAir`)
    (`KismetSystemLibrary.K2_SetTimerDelegate` (delegate `AntiAirExplode`) (/ (`self.AntiAirDistance`) (`self.RocketSpeed`)))))

(event `self.ReceiveTick`
  (params (DeltaSeconds :type "Float (single-precision)"))
  (bind _returnvalue (`self.K2_GetActorLocation`))
  (bind _array (`|MakeArray` null null null null :!type "Texture Object Reference"))
  (bind _returnvalue_2 (* (* (`self.GetActorForwardVector`) (`self.RocketSpeed`)) DeltaSeconds))
  (if (not (`self.Exploded`))
    ;[1 1 1] Trace from actual location to location in next frame
    (bind (_outhit _returnvalue_3) (`KismetSystemLibrary.SphereTraceSingle` _returnvalue (+ _returnvalue _returnvalue_2) 5.0 "TraceTypeQuery1" true (`|MakeArray` (`self.Instigator`) :!type "Actor Object Reference")))
    (if _returnvalue_3
      (bind (_bblockinghit _binitialoverlap _time _distance _location _impactpoint _normal _impactnormal _physmat _hitactor _hitcomponent) (`GameplayStatics.BreakHitResult` _outhit))
      ;[1 1 1] If hited another rocket - explode
      (bind _asbp_rocket_main (cast `/Game/BP/AI/Turret/BP_RocketMain` _hitactor)
        (:`then`
          (set `/Game/BP/AI/Turret/BP_RocketMain.AirPoof?` true _asbp_rocket_main)
          (bind _returnvalue_4 (`KismetMathLibrary.Conv_VectorToRotator` _normal))
          (`self.Explode` _asbp_rocket_main self _returnvalue_4 (`self.K2_GetActorLocation`) _outhit false))
        (:`CastFailed`
          _))
      ;[1 1 1] Create decal
      (if (`self.Decal?`)
        (if (!= (`GameplayStatics.GetObjectClass` _hitactor) "/Script/Engine.Pawn")
          (bind _output_get (set `self.DecalSize` (`KismetMathLibrary.RandomFloatInRange` 200.0 300.0)))
          (bind _returnvalue_5 (`GameplayStatics.SpawnDecalAttached` "/Game/Materials/MI_BoomDecal.MI_BoomDecal" (`KismetMathLibrary.MakeVector` 100.0 _output_get _output_get) _hitcomponent "None" _impactpoint _returnvalue_4 "KeepWorldPosition" 20.0))
          (`/Engine/EditorBlueprintResources/StandardMacros.IsValid` _returnvalue_5
            (:`Is Valid`
              (bind _returnvalue_6 (`DecalComponent.CreateDynamicMaterialInstance` _returnvalue_5))
              (bind _output_get_2 (set `self.DecalMat` _returnvalue_6))
              (`MaterialInstanceDynamic.SetTextureParameterValue` _output_get_2 "Decal_texture" (`|GetArrayItem` _array (`KismetMathLibrary.RandomIntegerInRange` 0 (`KismetArrayLibrary.Array_LastIndex` _array))))
              (`DecalComponent.SetDecalMaterial` _returnvalue_5 (`self.DecalMat`)))
            (:`Is Not Valid`
              _))))
      (`self.Explode` _hitactor _returnvalue_4 _impactpoint _outhit) ; Explode
      (else
        (`self.K2_AddActorWorldOffset` _returnvalue_2)))))

(event `self.ReceivePointDamage`
  (params (Damage :type "Float (single-precision)") (DamageType :type "DamageType Object Reference") (HitLocation :type "Vector Structure") (HitNormal :type "Vector Structure") (HitComponent :type "PrimitiveComponent Object Reference") (BoneName :type Name) (ShotFromDirection :type "Vector Structure") (InstigatedBy :type "Controller Object Reference") (DamageCauser :type "Actor Object Reference") (HitInfo :type "HitResult Structure (by ref)"))
  ;[1 1 1] Explode if get point damage
  (if (not (`self.Exploded`))
    (`self.ShowAll` HitNormal HitInfo)))

(event `ShowAll`
  (params (InVec :type "Vector Structure") (HitInfo :type "HitResult Structure"))
  (set `self.AirPoof?` true)
  (`self.Explode` null (`KismetMathLibrary.Conv_VectorToRotator` InVec) (`self.K2_GetActorLocation`) HitInfo true))

(fn `Explode`
  (params (`Other Actor` :type "Actor Object Reference") (Rotation :type "Rotator Structure") (Origin :type "Vector Structure") (HitInfo :type "HitResult Structure") (`AirExplode?` :type Boolean))
  (locals (RadialForce :type "RadialForceComponent Object Reference"))
  (bind _returnvalue (`self.K2_GetActorLocation`))
  (bind (_bblockinghit _binitialoverlap _time _distance _location _impactpoint _normal _impactnormal _physmat _hitactor _hitcomponent _hitbonename _hititem _faceindex _tracestart _traceend) (`GameplayStatics.BreakHitResult` HitInfo))
  (bind _attachvisibleaftercollide (`self.AttachVisibleAfterCollide`))
  (bind _radialforce (`self.RadialForce`))
  (bind _returnvalue_2 (/ (.x (`.BoxExtent` (`self.GetActorBounds` true))) 2.5))
  ;[1 1 1] If another actor not a instigator
  (if (and (!= `Other Actor` (`self.GetInstigator`)) (not (`self.Exploded`)))
    (set `self.Exploded` true)
    (if `AirExplode?`
      ;[1 1 1] Create impulse
      (set `RadialForceComponent.Radius` (`self.ExplodeRadius`) _radialforce :!label _label)
      (set `RadialForceComponent.ImpulseStrength` (`self.ImpulseStrength`) _radialforce)
      (`RadialForceComponent.FireImpulse` _radialforce)
      ;[1 1 1] Apply radial damage
      (`GameplayStatics.ApplyRadialDamageWithFalloff` :`BaseDamage` (`self.ExlodeDamage`) :`Origin` Origin :`DamageOuterRadius` (`self.ExplodeRadius`) :`DamageFalloff` (`self.Falloff`) :`DamageCauser` self :`InstigatedByController` null)
      (else
        ;[1 1 1] Apply damage from hit something
        (`GameplayStatics.ApplyPointDamage` `Other Actor` (`self.PointDamage`) (`KismetMathLibrary.Normal` (- _traceend _tracestart)) HitInfo null self)
        (if (`SceneComponent.IsSimulatingPhysics` _hitcomponent "None")
          (`PrimitiveComponent.AddImpulse` _hitcomponent (* (`self.GetActorForwardVector`) (`self.ImpulseStrength`)) "None" false))
        ;[1 1 1] Rocket have radial damage?
        (if (`self.RadialDamage?`)
          (goto _label)
          (else
            _))))
    (if (`self.Poof?`)
      ;[1 1 1] Spawn emitter
      (bind _returnvalue_3 (`GameplayStatics.SpawnEmitterAtLocation` (select `bool` (`self.AirPoof?`) :`false` (`self.GroundExplosion`) :`true` (`self.AirExplosion`)) _returnvalue Rotation))
      (`PrimitiveComponent.SetCastShadow` _returnvalue_3 false))
    (`GameplayStatics.PlaySoundAtLocation` (`self.ExplosionSound`) _returnvalue (struct) 1.0 1.0 0.0 null null null)
    (`self.SetLifeSpan` (`self.LifeAfterCollide`))
    (`SceneComponent.SetVisibility` (`self.Mesh`) _attachvisibleaftercollide false) ; Hide mesh
    ;[1 1 1] Attach actor after hit? Like nails
    (if _attachvisibleaftercollide
      (`self.K2_SetActorLocation` (+ Origin (* (`self.GetActorForwardVector`) (`KismetMathLibrary.RandomFloatInRange` (* _returnvalue_2 -1.0) _returnvalue_2))))
      (`self.K2_AttachToComponent` _hitcomponent "None" "KeepWorld" "KeepWorld" "KeepWorld"))
    ;[1 1 1] Disable collision
    (`PrimitiveComponent.SetCollisionEnabled` (`self.StaticMesh`) "NoCollision")
    (`PrimitiveComponent.SetCollisionEnabled` (`self.Mesh`) "NoCollision")))

(fn `UserConstructionScript`)