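; BP_RocketTurretAntiAir is an AI anti-air rocket turret that targets actors tagged Player.
; On BeginPlay it initializes its AITurretComponent with the roller and turret parts, two shoot points, a beam and an overlap sphere.
; The Init call also sets ranges, pitch limits, free rotation and burst timing, leaving aiming and firing to the component.
; The Blueprint adds no other logic of its own.
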(event `self.ReceiveTick`
  (params (DeltaSeconds :type "Float (single-precision)"))
  (`parent.ReceiveTick` DeltaSeconds))

(event `self.ReceiveBeginPlay`
  (`parent.ReceiveBeginPlay`)
  ;[1 1 1] Init turret
  (`/Game/BP/AI/Turret/BP_AITurretComponent.Init` (`self.AITurretComponent`) false (`self.Roller`) (`self.TurretContainer`) (`|MakeArray` (`self.ShootPos`) (`self.ShootPos1`)) (`self.Beam`) 8000.0 7000.0 false -20.0 85.0 15.0 1 true true false 0.3 self false 2 0.1 false (`self.OverlapSphere`) "Player"))

(fn `UserConstructionScript`
  (`parent.UserConstructionScript`))