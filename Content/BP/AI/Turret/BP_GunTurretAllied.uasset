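; BP_GunTurretAllied is an allied AI gun turret that can be damaged and destroyed.
; On BeginPlay it hands its meshes, two shoot points, beam, overlap sphere and target tag to AITurretComponent, configured for long-range, free-rotating burst fire.
; AnyDamage reduces Hp; at zero it marks the component as dead, spawns a small frag explosion at the turret and destroys the actor.
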(event `self.ReceiveTick`
  (params (DeltaSeconds :type "Float (single-precision)"))
  (`parent.ReceiveTick` DeltaSeconds))

(event `self.ReceiveBeginPlay`
  (`parent.ReceiveBeginPlay`)
  ;[1 1 1] Init turret
  (`/Game/BP/AI/Turret/BP_AITurretComponent.Init` (`self.AITurretComponent`) false (`self.Roller`) (`self.TurretContainer`) (`|MakeArray` (`self.ShootPos`) (`self.ShootPos1`)) (`self.Beam`) 40000.0 40000.0 false 0.0 320.0 5000.0 0 true false false 0.22 self false 4 0.2 false (`self.OverlapSphere`) (`self.TragetTag`)))

(event `self.ReceiveAnyDamage`
  (params (Damage :type "Float (single-precision)") (DamageType :type "DamageType Object Reference") (InstigatedBy :type "Controller Object Reference") (DamageCauser :type "Actor Object Reference"))
  (bind _output_get (set `self.Hp` (- (`self.Hp`) Damage)))
  (if (<= _output_get 0.0)
    (set `/Game/BP/AI/Turret/BP_AITurretComponent.IsAlive` false (`self.AITurretComponent`))
    (`GameplayStatics.SpawnEmitterAtLocation` "/Game/BallisticsVFX/Particles/Explosive/Explosion_Frag_small.Explosion_Frag_small" (.location (`SceneComponent.K2_GetComponentToWorld` (`self.TurretContainer`))) (.rotation (`SceneComponent.K2_GetComponentToWorld` (`self.TurretContainer`))) (.scale (`SceneComponent.K2_GetComponentToWorld` (`self.TurretContainer`))))
    (`self.K2_DestroyActor`)))

(fn `UserConstructionScript`
  (`parent.UserConstructionScript`))