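; AI turret component that finds, tracks and fires on tagged targets, optionally intercepting their rockets, with settings and parts supplied through Init.
; Each tick it drives an optional beam and free-rotates or aims the yaw roller and pitch-clamped turret.
; The server acquires targets by overlap sphere and visibility trace, while timers revalidate them and predict lead for rockets.
; Once aimed within range, it fires bullets or rockets as single, burst or random shots.
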(event `Init`
  (params (ResetInit :type Boolean) (Roller :type "StaticMeshComponent Object Reference") (Turret :type "StaticMeshComponent Object Reference") (SecondaryWeapPoints :type "Array of SceneComponent Object Reference") (Beam :type "ParticleSystemComponent Object Reference") (CheckRange :type "Float (double-precision)") (AttackRange :type "Float (double-precision)") (InvertRotator :type Boolean) (MinPitch :type "Float (double-precision)") (MaxPitch :type "Float (double-precision)") (GunRotationSpeed :type "Float (double-precision)") (AttackType :type Integer) (FreeRotation :type Boolean) (AntiAir :type Boolean) (AntiRocket :type Boolean) (TimeBetweenAttacks :type "Float (double-precision)" :default 0.8) (CharacterMain :type "Actor Object Reference") (BurstShot :type Boolean) (BurstShotCount :type Integer :default 2) (BurstShotDelay :type "Float (double-precision)" :default 0.2) (RandomShots :type Boolean) (OverlapSphere :type "StaticMeshComponent Object Reference") (TargetTag :type Name))
  (bind _beam (`self.Beam`))
  (bind _curtarget (`self.CurTarget`))
  (bind _searchclasses_ (`self.SearchClasses `))
  (bind _returnvalue (`SceneComponent.K2_GetComponentLocation` _beam))
  (bind _returnvalue_2 (+ (`self.Delta`) (`GameplayStatics.GetWorldDeltaSeconds`)))
  (bind _returnvalue_3 (+ _returnvalue (* (`SceneComponent.GetForwardVector` _beam) (`self.CheckRange`))))
  ;[1 1 1] Save variables
  (if ResetInit
    (`|ExecutionSequence`
      (:`then_0`
        (goto _label :!via `Reset`))
      (:`then_1`
        _)))
  (`/Engine/EditorBlueprintResources/StandardMacros.DoOnce` false :!label _label
    (:`Completed`
      (set `self.Roller` Roller)
      (set `self.Turret` Turret)
      (set `self.SecondaryWeapPoints` SecondaryWeapPoints)
      (set `self.Beam` Beam)
      (set `self.CheckRange` CheckRange)
      (set `self.AttackRange` AttackRange)
      (set `self.InvertRotator` InvertRotator)
      (set `self.MinPitch` MinPitch)
      (set `self.MaxPitch` MaxPitch)
      (set `self.GunRotationSpeed` GunRotationSpeed)
      (set `self.AttackType` AttackType)
      (set `self.FreeRotation` FreeRotation)
      (set `self.AntiAir` AntiAir)
      (set `self.AntiRocket` AntiRocket)
      (set `self.TimeBetweenAttacks` TimeBetweenAttacks)
      (set `self.CharacterMain` CharacterMain)
      (set `self.BurstShot` BurstShot)
      (set `self.BurstShotCount` BurstShotCount)
      (set `self.BurstShotDelay` BurstShotDelay)
      (set `self.RandomShots` RandomShots)
      (set `self.TargetTag` TargetTag)
      (`|ExecutionSequence`
        (:`then_0`
          ;[1 1 1] Set overlap sphere size
          (bind _output_get (set `self.OverlapSphere` OverlapSphere))
          (`SceneComponent.SetRelativeScale3D` _output_get (`KismetMathLibrary.Conv_DoubleToVector` (/ (`self.CheckRange`) 100.0)))
          ;[1 1 1] Set random start rotation
          (bind _turret (`self.Turret`)
            (:`then`
              (`SceneComponent.K2_SetRelativeRotation` _turret (`KismetMathLibrary.MakeRotator` 0.0 (`KismetMathLibrary.RandomFloatInRange` (`self.MinPitch`) (`self.MaxPitch`))) false true))
            (:`else`
              _))
          (bind _roller (`self.Roller`)
            (:`then`
              (`SceneComponent.K2_SetRelativeRotation` _roller (`KismetMathLibrary.MakeRotator` 0.0 0.0 (`KismetMathLibrary.RandomFloatInRange` 0.0 360.0)) false true))
            (:`else`)))
        (:`then_1`
          ;[1 1 1] Ignore self when find enemy
          (if (!= (`self.CharacterMain`) (`self.GetOwner`))
            (set `self.ActorsToIgnore` (`|MakeArray` (`self.CharacterMain`) (`self.GetOwner`)))
            (else
              (set `self.ActorsToIgnore` (`|MakeArray` (`self.CharacterMain`))))))
        (:`then_2`
          ;[1 1 1] Change classes to search if anti rocket
          (if (`self.AntiRocket`)
            (`KismetArrayLibrary.Array_Add` _searchclasses_ "/Game/BP/AI/Turret/BP_RocketMain.BP_RocketMain_C"))
          (`KismetArrayLibrary.Array_Add` _searchclasses_ "/Script/Engine.Actor"))
        (:`then_4`
          (goto _label_3 :!via `Open`))))))

(event `BurstShotAttack`
  ;[1 1 1] Burst attack
  (set `self.BurstShotCountCur` 0)
  (if (< (`self.BurstShotCountCur`) (`self.BurstShotCount`)) :!label _label_2
    (`/Engine/EditorBlueprintResources/StandardMacros.IncrementInt` (`self.BurstShotCountCur`)
      (:`  `
        (`self.Attack`)
        (set `self.LastAttack` (`KismetSystemLibrary.GetGameTimeInSeconds`))
        (`KismetSystemLibrary.Delay` (`self.BurstShotDelay`))
        (goto _label_2)))))

(event `self.ReceiveTick`
  (params (DeltaSeconds :type "Float (single-precision)"))
  (bind _beam (`self.Beam`))
  (bind _curtarget (`self.CurTarget`))
  (bind _returnvalue (`SceneComponent.K2_GetComponentLocation` _beam))
  (bind _returnvalue_2 (+ (`self.Delta`) (`GameplayStatics.GetWorldDeltaSeconds`)))
  (bind _returnvalue_3 (+ _returnvalue (* (`SceneComponent.GetForwardVector` _beam) (`self.CheckRange`))))
  (`/Engine/EditorBlueprintResources/StandardMacros.Gate` true :!label _label_3
    (:`Exit`
      (`/Engine/EditorBlueprintResources/StandardMacros.IsValid` _beam
        (:`Is Valid`
          (`/Engine/EditorBlueprintResources/StandardMacros.IsValid` (`self.CurTarget`)
            (:`Is Valid`
              (bind (_outhit _returnvalue_4) (`KismetSystemLibrary.LineTraceSingle` _returnvalue (`self.TargetOrigin`) "TraceTypeQuery1"))
              (`ParticleSystemComponent.SetBeamTargetPoint` _beam 0 (select `bool` (< (`self.CurDistanceToTarget`) 1000.0) :`false` _returnvalue_3 :`true` (select `bool` _returnvalue_4 :`false` _returnvalue_3 :`true` (`.Location` (`GameplayStatics.BreakHitResult` _outhit)))) 0))
            (:`Is Not Valid`
              (bind (_outhit_2 _returnvalue_5) (`KismetSystemLibrary.LineTraceSingle` _returnvalue _returnvalue_3 "TraceTypeQuery1"))
              (`ParticleSystemComponent.SetBeamTargetPoint` _beam 0 (select `bool` _returnvalue_5 :`false` _returnvalue_3 :`true` (`.Location` (`GameplayStatics.BreakHitResult` _outhit_2))) 0))))
        (:`Is Not Valid`
          _))
      ;[1 1 1] Target valid?
      (if (`KismetSystemLibrary.IsValid` _curtarget)
        ;[1 1 1] Get target origin
        (set `self.TargetOrigin` (`Actor.GetActorBounds` _curtarget true))
        (`|ExecutionSequence`
          (:`then_0`
            (goto _label_4 :!via `Reset`))
          (:`then_1`
            (`/Engine/EditorBlueprintResources/StandardMacros.IsValid` _beam
              (:`Is Valid`
                _)
              (:`Is Not Valid`
                _))
            ;[1 1 1] Used to predict target position
            (if (not (`KismetSystemLibrary.K2_TimerExists` null "Prediction"))
              (`KismetSystemLibrary.K2_SetTimer` null "Prediction" 0.05 true))
            (set `self.CurRange` (`KismetMathLibrary.VSize` (- (`Actor.K2_GetActorLocation` (`self.CharacterMain`)) (`Actor.K2_GetActorLocation` (`self.CurTarget`))))) ; Calculate range to target
            (if (not (`KismetSystemLibrary.K2_TimerExists` null "CheckTargetAndRemove"))
              ;[1 1 1] Check target state
              (`KismetSystemLibrary.K2_SetTimer` null "CheckTargetAndRemove" 0.5 true))
            ;[1 1 1] Not in attack range?
            (if (> (`self.CurRange`) (`self.AttackRange`))
              ;[1 0.6443 0] OnlyCheck
              (`KismetSystemLibrary.K2_ClearTimer` null "Attack")
              ;;[1 1 1] LostTarget
              (if (> (`self.CurRange`) (`self.CheckRange`))
                (set `self.CurTarget` null)
                (`KismetSystemLibrary.K2_ClearTimer` null "Prediction")
                (else
                  (`self.UpdateGunRotation`)))
              (else
                ;[1 0 0] Attack
                (`self.UpdateGunRotation`)
                (if (< (`self.CurDistanceToTarget`) 150.0)
                  (if (> (- (`KismetSystemLibrary.GetGameTimeInSeconds`) (`self.LastAttack`)) (`self.TimeBetweenAttacks`))
                    (set `self.LastAttack` (`KismetSystemLibrary.GetGameTimeInSeconds`))
                    (if (`self.RandomShots`)
                      (`self.RandomAttack`)
                      (elif (`self.BurstShot`)
                        (`self.BurstShotAttack`)
                        (else
                          (`self.Attack`))))))))))
        (else
          ;[1 1 1] Rotate freely when the target is not in sight
          (if (`self.FreeRotation`)
            (`self.FreeRotate`))
          (`|ExecutionSequence`
            (:`then_0`
              (`/Engine/EditorBlueprintResources/StandardMacros.DoOnce` false :!label _label_4
                (:`Completed`
                  (`KismetSystemLibrary.K2_ClearTimer` null "CheckTargetAndRemove")
                  (`KismetSystemLibrary.K2_ClearTimer` null "Attack")
                  (`KismetSystemLibrary.K2_ClearTimer` null "Prediction"))))
            (:`then_1`
              ;[1 1 1] Cooldown for get targets
              (if (`Actor.HasAuthority` (`self.CharacterMain`))
                (if (> _returnvalue_2 0.5)
                  (set `self.Delta` 0.0)
                  ;[1 1 1] Get actors in overlap sphere
                  (for _array_element (`self.SearchClasses `) :!label _label_5
                    (for _array_element_2 (`PrimitiveComponent.GetOverlappingActors` (`self.OverlapSphere`) _array_element)
                      (if (`Actor.ActorHasTag` _array_element_2 (`self.TargetTag`))
                        (bind (_visible _target) (`self.CheckTarget` _array_element_2 :!label _label_6)) ; Trace to target
                        (if (and _visible (`Actor.HasAuthority` (`self.GetOwner`)))
                          (set `self.CurTarget` _target)
                          (`|ExecutionSequence`
                            (:`then_0`
                              (break))
                            (:`then_1`
                              (goto _label_5 :!via `Break`))))
                        (elif (`self.AntiRocket`)
                          (bind (_asbp_rocket_main _bsuccess) (cast `/Game/BP/AI/Turret/BP_RocketMain` _array_element_2 :!pure true))
                          (if _bsuccess
                            (if (and (`Actor.ActorHasTag` (`Actor.Instigator` _array_element_2) (`self.TargetTag`)) (not (`/Game/BP/AI/Turret/BP_RocketMain.Exploded` _asbp_rocket_main)))
                              (goto _label_6)))))))
                  (else
                    (set `self.Delta` _returnvalue_2)))))))))))

(event `Disable`
  (bind _beam (`self.Beam`))
  ;[1 1 1] Function for disable this turret
  (`KismetSystemLibrary.K2_ClearTimer` null "Attack")
  (`KismetSystemLibrary.K2_ClearTimer` null "Prediction")
  (`KismetSystemLibrary.K2_ClearTimer` null "CheckTargetAndRemove")
  (`/Engine/EditorBlueprintResources/StandardMacros.IsValid` _beam
    (:`Is Valid`
      (`SceneComponent.SetVisibility` _beam false false)
      (goto _label_3 :!via `Close`))
    (:`Is Not Valid`
      (goto _label_3 :!via `Close`))))

(event `UpdateGunRotation`
  (bind _returnvalue (`GameplayStatics.GetWorldDeltaSeconds`))
  (bind _currange (`self.CurRange`))
  (bind _gunrotationspeed (`self.GunRotationSpeed`))
  (bind _turret (`self.Turret`))
  (bind _roller (`self.Roller`))
  (bind _returnvalue_2 (`SceneComponent.K2_GetComponentLocation` (`self.GetCurrentWeaponPoint`)))
  (bind _returnvalue_3 (`KismetMathLibrary.Square` _currange))
  (bind _returnvalue_4 (select `int` (`self.AttackType`) :`0` (`Actor.K2_GetActorLocation` (`self.CurTarget`)) :`1` (`self.NewPos`)))
  (bind _returnvalue_5 (`KismetMathLibrary.Conv_VectorToRotator` (`KismetMathLibrary.InverseTransformDirection` (`Actor.GetTransform` (`self.GetOwner`)) (`KismetMathLibrary.Conv_RotatorToVector` (select `bool` (`self.InvertRotator`) :`false` (`KismetMathLibrary.FindLookAtRotation` _returnvalue_2 _returnvalue_4) :`true` (`KismetMathLibrary.FindLookAtRotation` _returnvalue_4 _returnvalue_2))))))
  (bind _returnvalue_6 (`KismetMathLibrary.RInterpTo` (`KismetMathLibrary.MakeRotator` 0.0 0.0 (.yaw (`self.RollerRelative`))) (`KismetMathLibrary.MakeRotator` 0.0 0.0 (.yaw _returnvalue_5)) _returnvalue _gunrotationspeed))
  (bind _returnvalue_7 (`self.ClampPitch` (`KismetMathLibrary.RInterpTo` (`KismetMathLibrary.MakeRotator` 0.0 (.pitch (`self.TurretRelative`))) (`KismetMathLibrary.MakeRotator` 0.0 (.pitch _returnvalue_5)) _returnvalue _gunrotationspeed)))
  ;[1 1 1] Rotate turret
  (`/Engine/EditorBlueprintResources/StandardMacros.IsValid` _turret
    (:`Is Valid`
      (set `self.TurretRelative` (`SceneComponent.RelativeRotation` _turret))
      (`SceneComponent.K2_SetRelativeRotation` _turret _returnvalue_7 false true))
    (:`Is Not Valid`
      (set `self.TurretRelative` _returnvalue_7)))
  (`/Engine/EditorBlueprintResources/StandardMacros.IsValid` _roller
    (:`Is Valid`
      (set `self.RollerRelative` (`SceneComponent.RelativeRotation` _roller))
      (`SceneComponent.K2_SetRelativeRotation` _roller _returnvalue_6 false true))
    (:`Is Not Valid`
      (set `self.RollerRelative` _returnvalue_6)))
  (set `self.CurDistanceToTarget` (`KismetMathLibrary.Sqrt` (- (+ _returnvalue_3 _returnvalue_3) (* 2.0 _currange _currange (`KismetMathLibrary.DegCos` (`KismetMathLibrary.DegAcos` (`KismetMathLibrary.Dot_VectorVector` (`KismetMathLibrary.Conv_RotatorToVector` (`KismetMathLibrary.ComposeRotators` (`self.TurretRelative`) (`self.RollerRelative`))) (`KismetMathLibrary.Conv_RotatorToVector` (`KismetMathLibrary.MakeRotator` 0.0 (.pitch _returnvalue_5) (.yaw _returnvalue_5)))))))))))

(event `PrimWeapon`
  (params (Condition :type Boolean))
  (bind _weapontickdelay (`self.WeaponTickDelay`))
  ;[1 1 1] Attack with bullets
  (if Condition
    (if (not (`self.Shooted`))
      (set `self.Shooted` true)
      (`self.PrimaryWeaponTick`)
      (if (not (`KismetSystemLibrary.K2_TimerExists` null "PrimaryWeaponTick"))
        (`KismetSystemLibrary.K2_SetTimer` null "PrimaryWeaponTick" _weapontickdelay true)
        (`KismetSystemLibrary.Delay` _weapontickdelay)
        (set `self.Shooted` false))
      (else
        (`KismetSystemLibrary.K2_ClearTimer` null "PrimaryWeaponTick" :!label _label_7)))
    (else
      (goto _label_7))))

(fn `Attack`
  (locals (rocket :type "/Game/BP/AI/Turret/BP_Rocket1 Soft Class Reference"))
  (bind _curtarget (`self.CurTarget`))
  (if (`Actor.HasAuthority` (`self.CharacterMain`))
    (switch `int` (`self.AttackType`)
      (:`0`
        ;[1 1 1] Bullet weapon
        (`/Engine/EditorBlueprintResources/StandardMacros.IsValid` (`self.CurTarget`)
          (:`Is Valid`
            (`self.PrimaryWeaponTick`)
            (set `self.LastSecondaryPoint` (`.LastPointId` (`self.GetCurrentWeaponPoint`)))
            ;[1 1 1] If rocket is target - destroy
            (if (`self.AntiRocket`)
              (cast `/Game/BP/AI/Turret/BP_RocketMain` _curtarget)
              (`GameplayStatics.ApplyPointDamage` _curtarget 100.0 (0.0 0.0 0.0) (`GameplayStatics.MakeHitResult` false) null (`self.GetOwner`))
              (set `self.CurTarget` null)))))
      (:`1`
        ;[1 1 1] Rocket weapon
        (`self.SecondaryWeapon`)
        (set `self.LastSecondaryPoint` (`.LastPointId` (`self.GetCurrentWeaponPoint`)))))))

(fn `CheckTarget`
  (params (`Target 1` :type "Actor Object Reference"))
  (returns (Visible :type Boolean) (Target :type "Actor Object Reference"))
  ;[1 1 1] Trace from current weapon point to target
  (if (not (not (`KismetSystemLibrary.IsValid` `Target 1`)))
    (bind (_outhit _returnvalue) (`KismetSystemLibrary.SphereTraceSingle` (`SceneComponent.K2_GetComponentLocation` (`self.GetCurrentWeaponPoint`)) (`Actor.K2_GetActorLocation` `Target 1`) 5.0 "TraceTypeQuery1" true (`self.ActorsToIgnore`) "None" true (struct :`R` 1.0 :`A` 1.0) (struct :`G` 1.0 :`A` 1.0) 0.2))
    (if _returnvalue
      (bind (_bblockinghit _binitialoverlap _time _distance _location _impactpoint _normal _impactnormal _physmat _hitactor) (`GameplayStatics.BreakHitResult` _outhit))
      (bind _pitch (.pitch (`KismetMathLibrary.FindLookAtRotation` (0.0 0.0 0.0) (`KismetMathLibrary.InverseTransformLocation` (`SceneComponent.K2_GetComponentToWorld` (`self.Roller`)) (`Actor.K2_GetActorLocation` _hitactor)))))
      (return (and (< _pitch (`self.MaxPitch`)) (> _pitch (`self.MinPitch`)) (and (== `Target 1` _hitactor) (< (`KismetMathLibrary.VSize` (- (`Actor.K2_GetActorLocation` (`self.GetOwner`)) (`Actor.K2_GetActorLocation` `Target 1`))) (`self.CheckRange`)))) `Target 1`)
      (else
        _)))
  (return false `Target 1`))

(fn `CheckTargetAndRemove`
  (bind _curtarget (`self.CurTarget`))
  ;[1 1 1] Clear variable if target is not valid
  (`/Engine/EditorBlueprintResources/StandardMacros.IsValid` _curtarget
    (:`Is Valid`
      ;[1 1 1] Chect target range
      (bind (_outhit _returnvalue) (`KismetSystemLibrary.SphereTraceSingle` (`SceneComponent.K2_GetComponentLocation` (`self.GetCurrentWeaponPoint`)) (`Actor.K2_GetActorLocation` _curtarget) 5.0 "TraceTypeQuery1" false (`self.ActorsToIgnore`)))
      (if _returnvalue
        (bind (_bblockinghit _binitialoverlap _time _distance _location _impactpoint _normal _impactnormal _physmat _hitactor) (`GameplayStatics.BreakHitResult` _outhit))
        (bind _pitch (.pitch (`KismetMathLibrary.FindLookAtRotation` (0.0 0.0 0.0) (`KismetMathLibrary.InverseTransformLocation` (`SceneComponent.K2_GetComponentToWorld` (`self.Roller`)) (`Actor.K2_GetActorLocation` _hitactor)))))
        ;[1 1 1] Remove if not all good
        (if (not (and (< _pitch (`self.MaxPitch`)) (> _pitch (`self.MinPitch`)) (== _hitactor (`self.CurTarget`))))
          (set `self.CurTarget` null :!label _label))
        (else
          (goto _label))))
    (:`Is Not Valid`
      (set `self.CurTarget` null))))

(fn `ClampPitch`
  (params (InRot :type "Rotator Structure"))
  (returns (ReturnValue :type "Rotator Structure"))
  ;[1 1 1] Clamp rotation
  (return (`KismetMathLibrary.MakeRotator` (.roll InRot) (`KismetMathLibrary.ClampAngle` (.pitch InRot) (`self.MinPitch`) (`self.MaxPitch`)) (.yaw InRot))))

(fn `FreeRotate`
  (bind _turret (`self.Turret`))
  (bind _rotateyplus (`self.RotateYPlus`))
  (bind (_relativerotation_roll _relativerotation_pitch) (`KismetMathLibrary.BreakRotator` (`SceneComponent.RelativeRotation` _turret)))
  ;[1 1 1] Rotate turret if target not available
  (`SceneComponent.K2_AddWorldRotation` (`self.Roller`) (`KismetMathLibrary.MakeRotator` 0.0 0.0 (* 15.0 (`GameplayStatics.GetWorldDeltaSeconds`))) false false)
  (if (select `bool` _rotateyplus :`false` (< _relativerotation_pitch (`self.MinPitch`)) :`true` (> _relativerotation_pitch (`self.MaxPitch`)))
    (set `self.RotateYPlus` (not (`self.RotateYPlus`))))
  (`SceneComponent.K2_AddRelativeRotation` _turret (`KismetMathLibrary.MakeRotator` 0.0 (* (select `bool` _rotateyplus :`false` -10.0 :`true` 10.0 :!type "Float (single-precision)") (`GameplayStatics.GetWorldDeltaSeconds`))) false false))

(fn `GetCurrentWeaponPoint`
  (returns (SceneComponent :type "SceneComponent Object Reference") (LastPointId :type Integer))
  (bind _secondaryweappoints (`self.SecondaryWeapPoints`))
  (bind _returnvalue (+ (`self.LastSecondaryPoint`) 1))
  (bind _returnvalue_2 (`KismetMathLibrary.SelectInt` 0 _returnvalue (>= _returnvalue (`KismetArrayLibrary.Array_Length` _secondaryweappoints))))
  ;[1 1 1] Get current scene component for weapon
  (return (`|GetArrayItem` _secondaryweappoints _returnvalue_2) _returnvalue_2))

(fn `Prediction`
  (bind _scenecomponent (`self.GetCurrentWeaponPoint`))
  (bind _targetorigin (`self.TargetOrigin`))
  (bind _returnvalue (/ (- _targetorigin (`self.TargetLocation`)) 0.05))
  (switch `int` (`self.AttackType`)
    (:`1`
      (`/Engine/EditorBlueprintResources/StandardMacros.IsValid` (`self.CurTarget`)
        (:`Is Valid`
          (set `self.TargetVelocity` _returnvalue)
          (set `self.TargetForwardSpeed` (`KismetMathLibrary.VSize` _returnvalue))
          (set `self.TargetLocation` _targetorigin)
          (set `self.NewPos` (+ (`self.TargetLocation`) (* (`self.TargetVelocity`) (/ (`KismetMathLibrary.VSize` (- (`self.TargetLocation`) (`SceneComponent.K2_GetComponentLocation` _scenecomponent))) (- 7000.0 (* (`self.TargetForwardSpeed`) (`KismetMathLibrary.Dot_VectorVector` (`KismetMathLibrary.Normal` (`KismetMathLibrary.Conv_RotatorToVector` (`KismetMathLibrary.FindLookAtRotation` (`SceneComponent.K2_GetComponentLocation` _scenecomponent) (`self.TargetLocation`)))) (`KismetMathLibrary.Normal` (`self.TargetVelocity`))))))))))))))

(fn `PrimaryWeaponTick`
  (bind _secondaryweappoints (`self.SecondaryWeapPoints`))
  ;[1 1 1] If turret not dead
  (if (not (`self.Dead`))
    ;[1 1 1] Create bullet and play sound
    (if (> (`KismetArrayLibrary.Array_Length` _secondaryweappoints) 0)
      (for _array_element _secondaryweappoints
        (`/Engine/EditorBlueprintResources/StandardMacros.IsValid` _array_element
          (:`Is Valid`
            (`SceneComponent.K2_SetWorldRotation` _array_element (`KismetMathLibrary.FindLookAtRotation` (`SceneComponent.K2_GetComponentLocation` _array_element) (`self.TargetOrigin`)) false false)
            (`self.SpawnBullet` (`self.TargetOrigin`))))))))

(fn `RandomAttack`
  ;[1 1 1] Random attack, regular shot or burst
  (if (`KismetMathLibrary.RandomBool`)
    (`self.Attack`)
    (else
      (set `self.BurstShotDelay` (`KismetMathLibrary.RandomFloatInRange` 0.1 0.4))
      (set `self.BurstShotCount` (`KismetMathLibrary.RandomIntegerInRange` 1 3))
      (`self.BurstShotAttack`))))

(fn `SecondaryWeapon`
  (bind _secondaryweappoints (`self.SecondaryWeapPoints`))
  (bind _returnvalue (+ (`self.LastSecondaryPoint`) 1))
  (bind _returnvalue_2 (`KismetMathLibrary.SelectInt` 0 _returnvalue (>= _returnvalue (`KismetArrayLibrary.Array_Length` _secondaryweappoints))))
  (bind _output (`|GetArrayItem` _secondaryweappoints _returnvalue_2))
  (bind _returnvalue_3 (`SceneComponent.K2_GetComponentLocation` _output))
  (if (not (`self.Dead`))
    ;[1 1 1] Create rocket and init their parameters
    (`self.SpawnSecondary` _returnvalue_3 (+ _returnvalue_3 (* (`SceneComponent.GetForwardVector` _output) 1000.0)) (`self.AntiAir`) (select `bool` (`self.AntiAir`) :`true` (`KismetMathLibrary.Abs` (`KismetMathLibrary.VSize` (- (`SceneComponent.K2_GetComponentLocation` (`self.GetCurrentWeaponPoint`)) (`self.NewPos`))))))
    (set `self.LastSecondaryPoint` _returnvalue_2) ; Change current weapon point
  ))

(fn `SpawnBullet`
  (params (Target :type "Vector Structure (by ref)"))
  ;[1 1 1] Create bullet
  (for _array_element (`|MakeArray` (`self.GetCurrentWeaponPoint`))
    (bind _returnvalue (`SceneComponent.K2_GetComponentLocation` _array_element))
    (bind _returnvalue_2 (`KismetMathLibrary.FindLookAtRotation` _returnvalue Target))
    (`SceneComponent.K2_SetWorldRotation` _array_element _returnvalue_2 false false)
    (bind _aspawn (cast `Pawn` (`self.GetOwner`)))
    (`|SpawnActorFromClass` "/Game/BP/AI/Turret/BP_Bullet.BP_Bullet_C" (`KismetMathLibrary.MakeTransform` _returnvalue _returnvalue_2) "AlwaysSpawn" "OverrideRootScale" null (`self.AttackRange`) _aspawn)))

(fn `SpawnSecondary`
  (params (From :type "Vector Structure (by ref)") (To :type "Vector Structure") (AntiAir :type Boolean) (AntiAirDistance :type "Float (double-precision)"))
  ;[1 1 1] Create rocket with parameters
  (bind _aspawn (cast `Pawn` (`self.GetOwner`)))
  (`|SpawnActorFromClass` "/Game/BP/AI/Turret/BP_Rocket1.BP_Rocket1_C" (`KismetMathLibrary.MakeTransform` From (`KismetMathLibrary.FindLookAtRotation` From To)) "AlwaysSpawn" "OverrideRootScale" null AntiAirDistance AntiAir _aspawn)
  (return))