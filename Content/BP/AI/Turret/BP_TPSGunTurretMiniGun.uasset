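; Minigun gun turret actor that targets actors tagged Player and can be damaged and destroyed.
; BeginPlay hands its meshes, muzzle points and burst-fire tuning to BPAITurretComponentGround, whose target toggles TurnCannon each Tick and clears on overlap exit.
; AnyDamage spawns one-time spark and steam emitters at health thresholds, which Tick keeps pinned to SpawnEmitter.
; Death spawns an explosion and destroys the emitters and actor.
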(event `self.ReceiveTick`
  (params (DeltaSeconds :type "Float (single-precision)"))
  (bind _emitter_50 (`self.Emitter_50`))
  (bind _emitter_15 (`self.Emitter_15`))
  (bind _emitter_70 (`self.Emitter_70`))
  (bind _spawnemitter (`self.SpawnEmitter`))
  (bind _returnvalue (`SceneComponent.K2_GetComponentLocation` _spawnemitter))
  (bind _returnvalue_2 (`SceneComponent.K2_GetComponentRotation` _spawnemitter))
  (`parent.ReceiveTick` DeltaSeconds)
  (`|ExecutionSequence`
    (:`then_0`
      (`|ExecutionSequence`
        (:`then_0`
          (`/Engine/EditorBlueprintResources/StandardMacros.IsValid` _emitter_50
            (:`Is Valid`
              (`SceneComponent.K2_SetWorldLocationAndRotation` _emitter_50 _returnvalue _returnvalue_2 false false))))
        (:`then_1`
          (`/Engine/EditorBlueprintResources/StandardMacros.IsValid` _emitter_70
            (:`Is Valid`
              (`SceneComponent.K2_SetWorldLocationAndRotation` _emitter_70 _returnvalue _returnvalue_2 false false))))
        (:`then_2`
          (`/Engine/EditorBlueprintResources/StandardMacros.IsValid` _emitter_15
            (:`Is Valid`
              (`SceneComponent.K2_SetWorldLocationAndRotation` _emitter_15 _returnvalue _returnvalue_2 false false))))))
    (:`then_1`
      (if (!= (`/Game/BP/AI/Turret/BP_AITurretComponentGround.CurTarget` (`self.BP_AITurretComponentGround`)) null)
        (set `self.TurnCannon` true)
        (else
          (set `self.TurnCannon` false))))))

(event `self.ReceiveBeginPlay`
  (`parent.ReceiveBeginPlay`)
  (set `self.Hp` (`self.MaxHp`))
  ;[1 1 1] Init turret
  (`/Game/BP/AI/Turret/BP_AITurretComponentGround.Init` (`self.BP_AITurretComponentGround`) false (`self.Roller`) (`self.TurretContainer`) (`|MakeArray` (`self.ShootPos`) (`self.ShootPos1`)) (`self.Beam`) 3500.0 3500.0 false -20.0 50.0 4.0 0 false false false 0.065 self true 25 1.2 false (`self.OverlapSphere`) "Player"))

(event `self.OverlapSphere.OnComponentEndOverlap`
  (params (OverlappedComponent :type "PrimitiveComponent Object Reference") (OtherActor :type "Actor Object Reference") (OtherComp :type "PrimitiveComponent Object Reference") (OtherBodyIndex :type Integer))
  (if (`KismetSystemLibrary.IsValid` (`/Game/BP/AI/Turret/BP_AITurretComponentGround.CurTarget` (`self.BP_AITurretComponentGround`)))
    (set `/Game/BP/AI/Turret/BP_AITurretComponentGround.CurTarget` null (`self.BP_AITurretComponentGround`))))

(event `self.ReceiveAnyDamage`
  (params (Damage :type "Float (single-precision)") (DamageType :type "DamageType Object Reference") (InstigatedBy :type "Controller Object Reference") (DamageCauser :type "Actor Object Reference"))
  (bind _spawnemitter (`self.SpawnEmitter`))
  (bind _maxhp (`self.MaxHp`))
  (bind _returnvalue (`SceneComponent.K2_GetComponentLocation` _spawnemitter))
  (bind _returnvalue_2 (`SceneComponent.K2_GetComponentRotation` _spawnemitter))
  (bind _returnvalue_3 (- (`self.Hp`) Damage))
  (if (< _returnvalue_3 0.0)
    (`self.Death`)
    (else
      (bind _output_get (set `self.Hp` _returnvalue_3))
      (`|ExecutionSequence`
        (:`then_0`
          (if (<= _output_get (* _maxhp 0.5))
            (`/Engine/EditorBlueprintResources/StandardMacros.DoOnce` false
              (:`Completed`
                (bind _returnvalue_4 (`GameplayStatics.SpawnEmitterAtLocation` "/Game/PolygonCity/FX/P_FX_Steam1.P_FX_Steam1" _returnvalue _returnvalue_2))
                (set `self.Emitter_50` _returnvalue_4)))))
        (:`then_1`
          (if (<= _output_get (* _maxhp 0.3))
            (`/Engine/EditorBlueprintResources/StandardMacros.DoOnce` false
              (:`Completed`
                (bind _returnvalue_5 (`GameplayStatics.SpawnEmitterAtLocation` "/Game/PolygonCity/FX/P_FX_Steam2.P_FX_Steam2" _returnvalue _returnvalue_2))
                (set `self.Emitter_70` _returnvalue_5)))))
        (:`then_2`
          (if (<= _output_get (* _maxhp 0.85))
            (`/Engine/EditorBlueprintResources/StandardMacros.DoOnce` false
              (:`Completed`
                (bind _returnvalue_6 (`GameplayStatics.SpawnEmitterAtLocation` "/Game/LSS/DemoContent/SpaceshooterMinigame/Effects/P_Pixel_ExplosionimpactTurretSpark.P_Pixel_ExplosionimpactTurretSpark" _returnvalue _returnvalue_2))
                (set `self.Emitter_15` _returnvalue_6)))))))))

(event `Death`
  (bind (_returnvalue_location _returnvalue_rotation _returnvalue_scale) (`KismetMathLibrary.BreakTransform` (`self.GetTransform`)))
  (`GameplayStatics.SpawnEmitterAtLocation` "/Game/BallisticsVFX/Particles/Explosive/Explosion_GrenadeLauncher_2.Explosion_GrenadeLauncher_2" _returnvalue_location _returnvalue_rotation _returnvalue_scale)
  (`ActorComponent.K2_DestroyComponent` (`self.Emitter_50`))
  (`ActorComponent.K2_DestroyComponent` (`self.Emitter_70`))
  (`ActorComponent.K2_DestroyComponent` (`self.Emitter_15`))
  (`self.K2_DestroyActor`))

(fn `UserConstructionScript`
  (`parent.UserConstructionScript`))